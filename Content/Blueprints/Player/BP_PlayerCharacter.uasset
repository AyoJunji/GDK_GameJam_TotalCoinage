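; Player character for a timed scoring game in the CoinCity level, with movement, speed boost and landing slam.
; BeginPlay creates the HUD in that level, and events forward score, time and landing-triggered timer start to it.
; Boost temporarily raises walk speed, lengthens the camera arm and shows Niagara effects; hard landings fire a radial impulse.
; Tick eases mesh roll upright, and Deadzone overlaps deduct time and teleport the player to a fixed point.
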(event `self.ReceiveTick`
  (params (DeltaSeconds :type "Float (single-precision)"))
  (bind _staticmesh (`self.StaticMesh`))
  (bind (_returnvalue_roll _returnvalue_pitch _returnvalue_yaw) (`KismetMathLibrary.BreakRotator` (`SceneComponent.K2_GetComponentRotation` _staticmesh)))
  (bind _returnvalue (`SceneComponent.K2_GetComponentRotation` _staticmesh))
  (if (not (== _returnvalue (`KismetMathLibrary.MakeRotator` 0.0 _returnvalue_pitch _returnvalue_yaw)))
    (`SceneComponent.K2_SetWorldRotation` _staticmesh (`KismetMathLibrary.RInterpTo` _returnvalue (`KismetMathLibrary.MakeRotator` 0.0 _returnvalue_pitch _returnvalue_yaw) DeltaSeconds 1.0) false false)))

(event `self.OnLanded`
  (params (Hit :type "HitResult Structure (by ref)"))
  ;[1 0 0.03615] Landing Slam
  (`|ExecutionSequence`
    (:`then_0`
      (if (> (`KismetMathLibrary.VSize` (`MovementComponent.Velocity` (`self.CharacterMovement`))) 1200.0)
        (`RadialForceComponent.FireImpulse` (`self.RadialForce`))
        (`GameplayStatics.PlaySoundAtLocation` "/Game/Sounds/Sound_FX/Landing.Landing" (`self.K2_GetActorLocation`) (struct) 0.3 0.9 0.0 null null null null)
        (`ActorComponent.Activate` (`self.Niagara2`) true)))
    (:`then_1`
      (if (`self.StartTimer?`)
        (`/Game/Blueprints/Player/WB_PlayerHUD.CE_StartTimer` (`self.WB_PlayerHUD`))
        (set `self.StartTimer?` false)))))

(event `CE_BoostSpeed`
  (params (SpeedMutliplier :type "Float (double-precision)"))
  (bind _charactermovement (`self.CharacterMovement`))
  (bind _springarm (`self.SpringArm`))
  (bind _charactermovement_2 (`self.CharacterMovement`))
  (bind _springarm_2 (`self.SpringArm`))
  (bind _targetarmlength (`SpringArmComponent.TargetArmLength` _springarm))
  (bind _maxwalkspeed (`CharacterMovementComponent.MaxWalkSpeed` _charactermovement_2))
  (bind _targetarmlength_2 (`SpringArmComponent.TargetArmLength` _springarm_2))
  ;[0 1 0.2015] Change Speed
  (`SceneComponent.SetHiddenInGame` (`self.Niagara`) false false)
  (`SceneComponent.SetHiddenInGame` (`self.Niagara1`) false false)
  (set `self.isBoosting?` true)
  (`GameplayStatics.SpawnSoundAtLocation` "/Game/Sounds/Sound_FX/716972__newlocknew__expldsgn_engine-ignition-burstengine-startnitroflareblast.716972__newlocknew__expldsgn_engine-ignition-burstengine-startnitroflareblast" (`self.K2_GetActorLocation`) (struct) 0.1 0.9 0.0 null null)
  (set `CharacterMovementComponent.MaxWalkSpeed` (`KismetMathLibrary.FInterpTo` _maxwalkspeed (* SpeedMutliplier _maxwalkspeed) 1.0 1.0) _charactermovement_2)
  (set `SpringArmComponent.TargetArmLength` (`KismetMathLibrary.FInterpTo` _targetarmlength (+ _targetarmlength 200.0) 1.0 1.0) _springarm)
  (`KismetSystemLibrary.Delay` 10.0)
  (`SceneComponent.SetHiddenInGame` (`self.Niagara`) true false)
  (`SceneComponent.SetHiddenInGame` (`self.Niagara1`) true false)
  (set `self.isBoosting?` false)
  (set `CharacterMovementComponent.MaxWalkSpeed` (`KismetMathLibrary.FInterpTo` (`KismetMathLibrary.VSize` (`MovementComponent.Velocity` _charactermovement)) (`self.MaxSpeed`) 1.0 1.0) _charactermovement)
  (set `SpringArmComponent.TargetArmLength` (`KismetMathLibrary.FInterpTo` _targetarmlength_2 (+ _targetarmlength_2 -200.0) 1.0 1.0) _springarm_2))

(event `self.ReceiveBeginPlay`
  (bind _returnvalue (`GameplayStatics.GetCurrentLevelName` true))
  (if (`KismetStringLibrary.EqualEqual_StrStr` _returnvalue "CoinCity")
    ;[0 0.3179 1] Player HUD
    (`|ExecutionSequence`
      (:`then_0`
        (set `self.MaxSpeed` (`CharacterMovementComponent.MaxWalkSpeed` (`self.CharacterMovement`)))
        (`WidgetBlueprintLibrary.SetInputMode_GameOnly` (`GameplayStatics.GetPlayerController` 0)))
      (:`then_1`
        (bind _returnvalue_2 (`|CreateWidget` "/Game/Blueprints/Player/WB_PlayerHUD.WB_PlayerHUD_C"))
        (bind _output_get (set `self.WB_PlayerHUD` _returnvalue_2))
        (`UserWidget.AddToViewport` _output_get 0))
      (:`then_2`
        (if true
          (`GameplayStatics.PlaySoundAtLocation` "/Game/Sounds/Sound_FX/515311__matt_beer__tractor-motor-stopping.515311__matt_beer__tractor-motor-stopping" (`self.K2_GetActorLocation` self) (struct) 1.0 1.0 0.0 null null null null))))
    (else
      (`KismetSystemLibrary.PrintString` "Hello")
      (`WidgetBlueprintLibrary.SetInputMode_GameOnly` (`GameplayStatics.GetPlayerController` 0)))))

(event `ED_ChangeTime`
  (params (TimeToAdd :type "Float (double-precision)"))
  ;[0 0.3179 1] Player HUD
  (`/Game/Blueprints/Player/WB_PlayerHUD.CE_ChangeTime` (`self.WB_PlayerHUD`) TimeToAdd))

(event `EnhancedInput|/Game/Blueprints/Player/Input/IA_Movement`
  (params (ActionValue :type "Vector2D Structure") (ElapsedSeconds :type "Float (double-precision)") (TriggeredSeconds :type "Float (double-precision)") (InputAction :type "InputAction Object Reference" :default "/Game/Blueprints/Player/Input/IA_Movement.IA_Movement"))
  (:`Triggered`
    (`|ExecutionSequence`
      (:`then_0`
        (`self.AddMovementInput` (`self.GetActorRightVector`) ActionValue_X))
      (:`then_1`
        (`self.AddMovementInput` (`self.GetActorForwardVector`) ActionValue_Y)))))

(event `CE_ChangeScore`
  (params (ScoreAmount :type Integer))
  ;[1 1 1] Score
  (`/Game/Blueprints/Player/WB_PlayerHUD.CE_ChangeScore` (`self.WB_PlayerHUD`) ScoreAmount))

(event `self.Box.OnComponentBeginOverlap`
  (params (OverlappedComponent :type "PrimitiveComponent Object Reference") (OtherActor :type "Actor Object Reference") (OtherComp :type "PrimitiveComponent Object Reference") (OtherBodyIndex :type Integer) (bFromSweep :type Boolean) (SweepResult :type "HitResult Structure (by ref)"))
  (if (`self.ActorHasTag` OtherActor "Deadzone")
    (`/Game/Blueprints/Player/WB_PlayerHUD.CE_ChangeTime` (`self.WB_PlayerHUD`) -15.0)
    (`GameplayStatics.PlaySound2D` "/Game/Sounds/Sound_FX/253886__themusicalnomad__negative_beeps.253886__themusicalnomad__negative_beeps" 0.1 0.9 0.0 null null)
    (`self.K2_TeleportTo` (970.0 -1130.0 3850.0))))

(fn `UserConstructionScript`)
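; BP_ScoreZone is a score zone actor that animates two arrow markers, with no scoring logic in its graphs.
; On BeginPlay it starts two bounce events, each waiting DelayTime before playing its own timeline.
; Each timeline lerps an arrow's relative location vertically from a fixed height, the first toward the Distance variable and the second toward a lower fixed height.
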(event `CE_Bounce`
  (`KismetSystemLibrary.Delay` (`self.DelayTime`))
  (bind (_direction _newtrack_0) (`Timeline|Timeline`)
    (:`Update`
      (`SceneComponent.K2_SetRelativeLocation` (`self.Arrow`) (`KismetMathLibrary.VLerp` (0.0 0.0 6000.0) (`self.Distance`) _newtrack_0) false false))))

(event `self.ReceiveBeginPlay`
  (`self.CE_Bounce`)
  (`self.CE_Bounce2`))

(event `CE_Bounce2`
  (`KismetSystemLibrary.Delay` (`self.DelayTime`))
  (bind (_direction _newtrack_0) (`Timeline|Timeline_0`)
    (:`Update`
      (`SceneComponent.K2_SetRelativeLocation` (`self.Arrow1`) (`KismetMathLibrary.VLerp` (0.0 0.0 2500.0) (0.0 0.0 1250.0) _newtrack_0) false false))))

(fn `UserConstructionScript`)